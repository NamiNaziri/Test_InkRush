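; Ground environment actor that supports painting onto its static mesh through scene-capture rendering of an unwrap material.
; On BeginPlay it writes the capture ortho width and its location to the MPC_Global parameter collection and creates a dynamic M_Unwrap instance.
; PaintActor temporarily swaps in that material with hit location and brush radius, triggers a SceneCapture2D capture, then restores the original material.
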(event `self.ReceiveBeginPlay`
  (`KismetMaterialLibrary.SetScalarParameterValue` "/Game/Material/MPC_Global.MPC_Global" "CaptureSize" (`SceneCaptureComponent2D.OrthoWidth` (`self.SceneCaptureComponent2D`)))
  (`KismetSystemLibrary.PrintString` "Hello")
  (`KismetMaterialLibrary.SetVectorParameterValue` "/Game/Material/MPC_Global.MPC_Global" "UnwrapLocation" (`KismetMathLibrary.Conv_VectorToLinearColor` (`self.K2_GetActorLocation`)))
  (bind _returnvalue (`KismetMaterialLibrary.CreateDynamicMaterialInstance` "/Game/Material/M_Unwrap.M_Unwrap"))
  (set `self.Unwrap Material` _returnvalue))

(fn `PaintActor`
  (params (HitLocation :type "Vector Structure") (BrushRadius :type "Float (double-precision)") (ActorToCapture :type "Actor Object Reference"))
  (`|ExecutionSequence`
    (:`then_0`
      (set `self.OriginalMaterial` (`PrimitiveComponent.GetMaterial` (`self.StaticMesh`) 0))
      (`PrimitiveComponent.SetMaterial` (`self.StaticMesh`) 0 (`self.Unwrap Material`)))
    (:`then_1`
      (`MaterialInstanceDynamic.SetVectorParameterValue` (`self.Unwrap Material`) "HitLocation" (`KismetMathLibrary.Conv_VectorToLinearColor` HitLocation))
      (`MaterialInstanceDynamic.SetScalarParameterValue` (`self.Unwrap Material`) "BrushRadius" (`local.BrushRadius`)))
    (:`then_2`
      (`SceneCaptureComponent2D.CaptureScene` (`self.SceneCaptureComponent2D`))
      (`PrimitiveComponent.SetMaterial` (`self.StaticMesh`) 0 (`self.OriginalMaterial`)))))

(fn `UserConstructionScript`)