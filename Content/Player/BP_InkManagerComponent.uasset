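; Ink manager component that paints ink onto hit surfaces using render targets stored per actor name.
; The first hit creates an ink target sized from actor bounds plus an influence target, and binds the ink target to a dynamic surface material.
; Each hit derives brush position, scale and squish from collision UVs and tangential offset samples.
; Repeat hits draw cleanup then brush into the ink target, and brush into the influence target.
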(event `InitializeInkManager`
  (params (`Current Name` :type String) (RenderTargetWidth :type Integer) (RenderTargetHeight :type Integer) (ParentMaterial :type "MaterialInterface Object Reference") (HitComponent :type "PrimitiveComponent Object Reference") (`Brush uvTransform` :type "LinearColor Structure") (BrushScale :type "Float (single-precision)") (BrushSquish :type "LinearColor Structure"))
  (set `self.Current Name` `Current Name`)
  (`self.InitializeBrushes`)
  (`self.CreateRenderTargets` RenderTargetWidth RenderTargetHeight)
  (`self.SetMaterialInstanceAndRenderTarget` ParentMaterial HitComponent (`self.Current RT`))
  (`self.SetBrushParameters` (`self.Brush`) `Brush uvTransform` BrushScale BrushSquish)
  (`KismetRenderingLibrary.DrawMaterialToRenderTarget` (`self.Current RT`) (`self.Brush`))
  (`KismetRenderingLibrary.DrawMaterialToRenderTarget` (`BlueprintMapLibrary.Map_Find` (`self.Actor Name to Influence RT`) (`self.Current Name`)) (`self.Brush`)))

(event `Paint`
  (params (`Current Name` :type String) (Hit :type "HitResult Structure (by ref)"))
  (bind (_rendertargetdim _uvtransform _squish _scale) (`self.Calculate Brush Values` Hit))
  (bind (_bblockinghit _binitialoverlap _time _distance _location _impactpoint _normal _impactnormal _physmat _hitactor _hitcomponent) (`GameplayStatics.BreakHitResult` Hit))
  (bind (_rendertargetdim_2 _uvtransform_2 _squish_2 _scale_2) (`self.Calculate Brush Values` Hit))
  (bind _output_get (set `self.Current Name` `Current Name`))
  (if (`BlueprintMapLibrary.Map_Contains` (`self.Actor Name to RT`) _output_get)
    (set `self.Current RT` (`BlueprintMapLibrary.Map_Find` (`self.Actor Name to RT`) (`self.Current Name`)))
    (`self.SetBrushParameters` (`self.Cleanup`) _uvtransform_2 _scale_2 _squish_2)
    (`self.SetBrushParameters` (`self.Brush`) _uvtransform_2 _scale_2 _squish_2)
    (`KismetRenderingLibrary.DrawMaterialToRenderTarget` (`self.Current RT`) (`self.Cleanup`))
    (`KismetRenderingLibrary.DrawMaterialToRenderTarget` (`self.Current RT`) (`self.Brush`))
    (`KismetRenderingLibrary.DrawMaterialToRenderTarget` (`BlueprintMapLibrary.Map_Find` (`self.Actor Name to Influence RT`) (`self.Current Name`)) (`self.Brush`))
    (else
      (`self.InitializeInkManager` (`self.Current Name`) _rendertargetdim _rendertargetdim (`PrimitiveComponent.GetMaterial` _hitcomponent 0) _hitcomponent _uvtransform _scale _squish))))

(fn `Calculate Brush Values`
  (params (Hit :type "HitResult Structure (by ref)"))
  (returns (RenderTargetDim :type Integer) (uvTransform :type "LinearColor Structure") (squish :type "LinearColor Structure") (scale :type "Float (double-precision)"))
  (bind (_bblockinghit _binitialoverlap _time _distance _location _impactpoint _normal _impactnormal _physmat _hitactor _hitcomponent _hitbonename _bonename _hititem _elementindex _faceindex) (`GameplayStatics.BreakHitResult` Hit))
  (bind _uv (`GameplayStatics.FindCollisionUV` (`local.Hit`)))
  (bind _returnvalue (`KismetMathLibrary.Normal` (`KismetMathLibrary.Cross_VectorVector` (`KismetMathLibrary.RandomUnitVectorFromStream` (`KismetMathLibrary.MakeRandomStream` 0)) _normal)))
  (bind _returnvalue_2 (- (`GameplayStatics.FindCollisionUV` (`GameplayStatics.MakeHitResult` false false 0.0 0.0 (+ _location (* _returnvalue 25.0)) (0.0 0.0 0.0) (0.0 0.0 1.0) (0.0 0.0 1.0) null null _hitcomponent "None" "None" 0 0 _faceindex)) _uv))
  (bind _returnvalue_3 (- (`GameplayStatics.FindCollisionUV` (`GameplayStatics.MakeHitResult` false false 0.0 0.0 (+ _location (* (`KismetMathLibrary.Normal` (`KismetMathLibrary.Cross_VectorVector` _returnvalue _normal)) 25.0)) (0.0 0.0 0.0) (0.0 0.0 1.0) (0.0 0.0 1.0) null null _hitcomponent "None" "None" 0 0 _faceindex)) _uv))
  (return (`self.CalculateRenderTargetDim` _hitactor) (`KismetMathLibrary.Conv_VectorToLinearColor` (`KismetMathLibrary.Conv_Vector2DToVector` (`GameplayStatics.FindCollisionUV` (`local.Hit`)))) (`KismetMathLibrary.Conv_VectorToLinearColor` (`KismetMathLibrary.MakeVector` (`KismetMathLibrary.DotProduct2D` _returnvalue_2 (1.0 0.0)) (`KismetMathLibrary.DotProduct2D` _returnvalue_3 (0.0 1.0)))) (`KismetMathLibrary.VSize2D` (+ _returnvalue_2 _returnvalue_3))))

(fn `CalculateRenderTargetDim`
  (params (HitActor :type "Actor Object Reference"))
  (returns (ReturnValue :type Integer))
  (bind (_origin _boxextent) (`Actor.GetActorBounds` HitActor false false))
  (return (`KismetMathLibrary.FTrunc` (`KismetMathLibrary.MultiplyMultiply_FloatFloat` 2.0 (`KismetMathLibrary.Conv_IntToDouble` (`KismetMathLibrary.FTrunc` (`KismetMathLibrary.MapRangeClamped` (/ (* (+ (* (.x _boxextent) (.y _boxextent)) (* (.x _boxextent) (.z _boxextent)) (* (.y _boxextent) (.z _boxextent))) 8.0) 10000.0) 50.0 500.0 9.0 13.0)))))))

(fn `CreateRenderTargets`
  (params (RenderTargetWidth :type Integer) (RenderTargetHeight :type Integer))
  (bind _returnvalue (`KismetRenderingLibrary.CreateRenderTarget2D` RenderTargetWidth RenderTargetHeight "RTF_R16f" (struct :`A` 1.0) false true))
  (bind _output_get (set `self.Current RT` _returnvalue))
  (`BlueprintMapLibrary.Map_Add` (`self.Actor Name to RT`) (`self.Current Name`) _output_get)
  (bind _returnvalue_2 (`KismetRenderingLibrary.CreateRenderTarget2D` (`self.Influence Dim`) (`self.Influence Dim`) "RTF_RGBA8_SRGB" (struct :`A` 1.0) false true))
  (`BlueprintMapLibrary.Map_Add` (`self.Actor Name to Influence RT`) (`self.Current Name`) _returnvalue_2))

(fn `InitializeBrushes`
  (bind _returnvalue (`KismetMaterialLibrary.CreateDynamicMaterialInstance` "/Game/Material/M_Brush.M_Brush"))
  (set `self.Positive` _returnvalue)
  (bind _returnvalue_2 (`KismetMaterialLibrary.CreateDynamicMaterialInstance` "/Game/Material/M_Brush_N.M_Brush_N"))
  (set `self.Negative` _returnvalue_2)
  (bind _returnvalue_3 (`KismetMaterialLibrary.CreateDynamicMaterialInstance` "/Game/Material/M_Brush_CleanUp.M_Brush_CleanUp"))
  (set `self.Cleanup` _returnvalue_3)
  (set `self.Brush` (`self.Positive`)))

(fn `SetBrushParameters`
  (params (Brush :type "MaterialInstanceDynamic Object Reference") (uvTransform :type "LinearColor Structure") (scale :type "Float (single-precision)") (squish :type "LinearColor Structure"))
  (`MaterialInstanceDynamic.SetVectorParameterValue` Brush "uvTransform" uvTransform)
  (`MaterialInstanceDynamic.SetScalarParameterValue` (`local.Brush`) "scale" scale)
  (`MaterialInstanceDynamic.SetVectorParameterValue` (`local.Brush`) "squish" squish))

(fn `SetMaterialInstanceAndRenderTarget`
  (params (ParentMaterial :type "MaterialInterface Object Reference") (HitComponent :type "PrimitiveComponent Object Reference") (RenderTargetToSet :type "Texture Object Reference"))
  (bind _returnvalue (`KismetMaterialLibrary.CreateDynamicMaterialInstance` ParentMaterial))
  (`PrimitiveComponent.SetMaterial` HitComponent 0 _returnvalue)
  (`MaterialInstanceDynamic.SetTextureParameterValue` _returnvalue "InkRT" RenderTargetToSet))