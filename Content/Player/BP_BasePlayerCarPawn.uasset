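; Base player car pawn that paints ink onto the surface beneath it every tick, with debug keys switching between positive and negative brushes.
; A downward trace finds the hit UV, and offset UV samples along surface tangents set brush scale and squish.
; Each newly hit actor gets a bounds-sized render target bound to its material as InkRT.
; Later hits draw a cleanup material, then the brush, into that target.
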(event EventBeginPlay
  (|CallParentFunction)
  (Rendering|ClearRenderTarget2D "/Game/Material/RT_Capture.RT_Capture")
  (bind _returnvalue (Rendering|Material|CreateDynamicMaterialInstance "/Game/Material/M_Brush.M_Brush" "None" "None" :!class /Script/Engine.KismetMaterialLibrary))
  (Variables|Default|SetPositive _returnvalue)
  (bind _returnvalue_2 (Rendering|Material|CreateDynamicMaterialInstance "/Game/Material/M_Brush_N.M_Brush_N" "None" "None" :!class /Script/Engine.KismetMaterialLibrary))
  (Variables|Default|SetNegative _returnvalue_2)
  (bind _returnvalue_3 (Rendering|Material|CreateDynamicMaterialInstance "/Game/Material/M_Brush_CleanUp.M_Brush_CleanUp" "None" "None" :!class /Script/Engine.KismetMaterialLibrary))
  (Variables|Default|SetCleanup _returnvalue_3)
  (Variables|Default|SetBrush (Variables|Default|GetPositive)))

(event Collision|EventActorBeginOverlap
  (params (OtherActor :type Actor%20Object%20Reference)))

(event EventTick
  (params (DeltaSeconds :type Float%20%28single-precision%29))
  (bind _returnvalue (Transformation|GetActorLocation))
  (|CallParentFunction DeltaSeconds)
  (bind (_outhit _returnvalue_2) (Collision|LineTraceByChannel _returnvalue (+ _returnvalue (* (Transformation|GetActorUpVector) -5e+02)) "TraceTypeQuery1" true 0 "None"))
  (if _returnvalue_2
    (if (Utilities|Map|Contains (Variables|Default|GetActorNameToRT) (Utilities|GetObjectName (.HitActor (Collision|BreakHitResult _outhit))))
      (Rendering|Material|SetVectorParameterValue (Variables|Default|GetCleanup) "uvTransform" (Math|Conversions|ToLinearColor(Vector) (Math|Conversions|ToVector(Vector2D) (.UV (Class|GameplayStatics|FindCollisionUV _outhit)))) :!class /Script/Engine.MaterialInstanceDynamic)
      (Rendering|Material|SetScalarParameterValue (Variables|Default|GetCleanup) "scale" (Math|Vector2D|Vector2DLength (+ (- (.UV (Class|GameplayStatics|FindCollisionUV (Collision|MakeHitResult false false 0.0 0.0 (+ (.Location (Collision|BreakHitResult _outhit)) (* (Math|Vector|Normalize (Math|Vector|CrossProduct (Math|Random|RandomUnitVectorfromStream (Math|Random|MakeRandomStream 0)) (.Normal (Collision|BreakHitResult _outhit)))) 25.0)) "0, 0, 0" "0,0,1" "0,0,1" 0 0 (.HitComponent (Collision|BreakHitResult _outhit)) "None" "None" 0 0 (.FaceIndex (Collision|BreakHitResult _outhit))))) (.UV (Class|GameplayStatics|FindCollisionUV _outhit))) (- (.UV (Class|GameplayStatics|FindCollisionUV (Collision|MakeHitResult false false 0.0 0.0 (+ (.Location (Collision|BreakHitResult _outhit)) (* (Math|Vector|Normalize (Math|Vector|CrossProduct (Math|Vector|Normalize (Math|Vector|CrossProduct (Math|Random|RandomUnitVectorfromStream (Math|Random|MakeRandomStream 0)) (.Normal (Collision|BreakHitResult _outhit)))) (.Normal (Collision|BreakHitResult _outhit)))) 25.0)) "0, 0, 0" "0,0,1" "0,0,1" 0 0 (.HitComponent (Collision|BreakHitResult _outhit)) "None" "None" 0 0 (.FaceIndex (Collision|BreakHitResult _outhit))))) (.UV (Class|GameplayStatics|FindCollisionUV _outhit))))) :!class /Script/Engine.MaterialInstanceDynamic)
      (Rendering|Material|SetVectorParameterValue (Variables|Default|GetCleanup) "squish" (Math|Conversions|ToLinearColor(Vector) (Math|Vector|MakeVector (Math|Vector2D|DotProduct(2D) (- (.UV (Class|GameplayStatics|FindCollisionUV (Collision|MakeHitResult false false 0.0 0.0 (+ (.Location (Collision|BreakHitResult _outhit)) (* (Math|Vector|Normalize (Math|Vector|CrossProduct (Math|Random|RandomUnitVectorfromStream (Math|Random|MakeRandomStream 0)) (.Normal (Collision|BreakHitResult _outhit)))) 25.0)) "0, 0, 0" "0,0,1" "0,0,1" 0 0 (.HitComponent (Collision|BreakHitResult _outhit)) "None" "None" 0 0 (.FaceIndex (Collision|BreakHitResult _outhit))))) (.UV (Class|GameplayStatics|FindCollisionUV _outhit))) "(X=1.000000,Y=0.000000)") (Math|Vector2D|DotProduct(2D) (- (.UV (Class|GameplayStatics|FindCollisionUV (Collision|MakeHitResult false false 0.0 0.0 (+ (.Location (Collision|BreakHitResult _outhit)) (* (Math|Vector|Normalize (Math|Vector|CrossProduct (Math|Vector|Normalize (Math|Vector|CrossProduct (Math|Random|RandomUnitVectorfromStream (Math|Random|MakeRandomStream 0)) (.Normal (Collision|BreakHitResult _outhit)))) (.Normal (Collision|BreakHitResult _outhit)))) 25.0)) "0, 0, 0" "0,0,1" "0,0,1" 0 0 (.HitComponent (Collision|BreakHitResult _outhit)) "None" "None" 0 0 (.FaceIndex (Collision|BreakHitResult _outhit))))) (.UV (Class|GameplayStatics|FindCollisionUV _outhit))) "(X=0.000000,Y=1.000000)") 0.0)) :!class /Script/Engine.MaterialInstanceDynamic)
      (Rendering|Material|SetVectorParameterValue (Variables|Default|GetBrush) "uvTransform" (Math|Conversions|ToLinearColor(Vector) (Math|Conversions|ToVector(Vector2D) (.UV (Class|GameplayStatics|FindCollisionUV _outhit)))) :!class /Script/Engine.MaterialInstanceDynamic)
      (Rendering|Material|SetScalarParameterValue (Variables|Default|GetBrush) "scale" (Math|Vector2D|Vector2DLength (+ (- (.UV (Class|GameplayStatics|FindCollisionUV (Collision|MakeHitResult false false 0.0 0.0 (+ (.Location (Collision|BreakHitResult _outhit)) (* (Math|Vector|Normalize (Math|Vector|CrossProduct (Math|Random|RandomUnitVectorfromStream (Math|Random|MakeRandomStream 0)) (.Normal (Collision|BreakHitResult _outhit)))) 25.0)) "0, 0, 0" "0,0,1" "0,0,1" 0 0 (.HitComponent (Collision|BreakHitResult _outhit)) "None" "None" 0 0 (.FaceIndex (Collision|BreakHitResult _outhit))))) (.UV (Class|GameplayStatics|FindCollisionUV _outhit))) (- (.UV (Class|GameplayStatics|FindCollisionUV (Collision|MakeHitResult false false 0.0 0.0 (+ (.Location (Collision|BreakHitResult _outhit)) (* (Math|Vector|Normalize (Math|Vector|CrossProduct (Math|Vector|Normalize (Math|Vector|CrossProduct (Math|Random|RandomUnitVectorfromStream (Math|Random|MakeRandomStream 0)) (.Normal (Collision|BreakHitResult _outhit)))) (.Normal (Collision|BreakHitResult _outhit)))) 25.0)) "0, 0, 0" "0,0,1" "0,0,1" 0 0 (.HitComponent (Collision|BreakHitResult _outhit)) "None" "None" 0 0 (.FaceIndex (Collision|BreakHitResult _outhit))))) (.UV (Class|GameplayStatics|FindCollisionUV _outhit))))) :!class /Script/Engine.MaterialInstanceDynamic)
      (Rendering|Material|SetVectorParameterValue (Variables|Default|GetBrush) "squish" (Math|Conversions|ToLinearColor(Vector) (Math|Vector|MakeVector (Math|Vector2D|DotProduct(2D) (- (.UV (Class|GameplayStatics|FindCollisionUV (Collision|MakeHitResult false false 0.0 0.0 (+ (.Location (Collision|BreakHitResult _outhit)) (* (Math|Vector|Normalize (Math|Vector|CrossProduct (Math|Random|RandomUnitVectorfromStream (Math|Random|MakeRandomStream 0)) (.Normal (Collision|BreakHitResult _outhit)))) 25.0)) "0, 0, 0" "0,0,1" "0,0,1" 0 0 (.HitComponent (Collision|BreakHitResult _outhit)) "None" "None" 0 0 (.FaceIndex (Collision|BreakHitResult _outhit))))) (.UV (Class|GameplayStatics|FindCollisionUV _outhit))) "(X=1.000000,Y=0.000000)") (Math|Vector2D|DotProduct(2D) (- (.UV (Class|GameplayStatics|FindCollisionUV (Collision|MakeHitResult false false 0.0 0.0 (+ (.Location (Collision|BreakHitResult _outhit)) (* (Math|Vector|Normalize (Math|Vector|CrossProduct (Math|Vector|Normalize (Math|Vector|CrossProduct (Math|Random|RandomUnitVectorfromStream (Math|Random|MakeRandomStream 0)) (.Normal (Collision|BreakHitResult _outhit)))) (.Normal (Collision|BreakHitResult _outhit)))) 25.0)) "0, 0, 0" "0,0,1" "0,0,1" 0 0 (.HitComponent (Collision|BreakHitResult _outhit)) "None" "None" 0 0 (.FaceIndex (Collision|BreakHitResult _outhit))))) (.UV (Class|GameplayStatics|FindCollisionUV _outhit))) "(X=0.000000,Y=1.000000)") 0.0)) :!class /Script/Engine.MaterialInstanceDynamic)
      (Rendering|DrawMaterialtoRenderTarget (.Value (Utilities|Map|Find (Variables|Default|GetActorNameToRT) (Utilities|GetObjectName (.HitActor (Collision|BreakHitResult _outhit))))) (Variables|Default|GetCleanup))
      (Rendering|DrawMaterialtoRenderTarget (.Value (Utilities|Map|Find (Variables|Default|GetActorNameToRT) (Utilities|GetObjectName (.HitActor (Collision|BreakHitResult _outhit))))) (Variables|Default|GetBrush))
      (else
        (bind _returnvalue_3 (Rendering|CreateRenderTarget2D (Math|Float|Truncate (Math|Float|Power 2.0 (Math|Conversions|ToFloat(Integer) (Math|Float|Truncate (Math|Float|MapRangeClamped (/ (* (+ (* (.x (.BoxExtent (Collision|GetActorBounds (.HitActor (Collision|BreakHitResult _outhit)) false false))) (.y (.BoxExtent (Collision|GetActorBounds (.HitActor (Collision|BreakHitResult _outhit)) false false)))) (* (.x (.BoxExtent (Collision|GetActorBounds (.HitActor (Collision|BreakHitResult _outhit)) false false))) (.z (.BoxExtent (Collision|GetActorBounds (.HitActor (Collision|BreakHitResult _outhit)) false false)))) (* (.y (.BoxExtent (Collision|GetActorBounds (.HitActor (Collision|BreakHitResult _outhit)) false false))) (.z (.BoxExtent (Collision|GetActorBounds (.HitActor (Collision|BreakHitResult _outhit)) false false))))) 8.0) 1e+04) 5e+01 5e+02 9.0 13.0))))) (Math|Float|Truncate (Math|Float|Power 2.0 (Math|Conversions|ToFloat(Integer) (Math|Float|Truncate (Math|Float|MapRangeClamped (/ (* (+ (* (.x (.BoxExtent (Collision|GetActorBounds (.HitActor (Collision|BreakHitResult _outhit)) false false))) (.y (.BoxExtent (Collision|GetActorBounds (.HitActor (Collision|BreakHitResult _outhit)) false false)))) (* (.x (.BoxExtent (Collision|GetActorBounds (.HitActor (Collision|BreakHitResult _outhit)) false false))) (.z (.BoxExtent (Collision|GetActorBounds (.HitActor (Collision|BreakHitResult _outhit)) false false)))) (* (.y (.BoxExtent (Collision|GetActorBounds (.HitActor (Collision|BreakHitResult _outhit)) false false))) (.z (.BoxExtent (Collision|GetActorBounds (.HitActor (Collision|BreakHitResult _outhit)) false false))))) 8.0) 1e+04) 5e+01 5e+02 9.0 13.0))))) "RTF_R16f" "(R=0.000000,G=0.000000,B=0.000000,A=1.000000)" false true))
        (Utilities|Map|Add (Variables|Default|GetActorNameToRT) (Utilities|GetObjectName (.HitActor (Collision|BreakHitResult _outhit))) _returnvalue_3)
        (bind _returnvalue_4 (Rendering|Material|CreateDynamicMaterialInstance (Rendering|Material|GetMaterial (.HitComponent (Collision|BreakHitResult _outhit)) 0) "None" "None" :!class /Script/Engine.KismetMaterialLibrary))
        (Rendering|Material|SetMaterial (.HitComponent (Collision|BreakHitResult _outhit)) 0 _returnvalue_4)
        (Rendering|Material|SetTextureParameterValue _returnvalue_4 "InkRT" _returnvalue_3)
        (Rendering|Material|SetVectorParameterValue (Variables|Default|GetBrush) "uvTransform" (Math|Conversions|ToLinearColor(Vector) (Math|Conversions|ToVector(Vector2D) (.UV (Class|GameplayStatics|FindCollisionUV _outhit)))) :!class /Script/Engine.MaterialInstanceDynamic)
        (Rendering|Material|SetScalarParameterValue (Variables|Default|GetBrush) "scale" (Math|Vector2D|Vector2DLength (+ (- (.UV (Class|GameplayStatics|FindCollisionUV (Collision|MakeHitResult false false 0.0 0.0 (+ (.Location (Collision|BreakHitResult _outhit)) (* (Math|Vector|Normalize (Math|Vector|CrossProduct (Math|Random|RandomUnitVectorfromStream (Math|Random|MakeRandomStream 0)) (.Normal (Collision|BreakHitResult _outhit)))) 25.0)) "0, 0, 0" "0,0,1" "0,0,1" 0 0 (.HitComponent (Collision|BreakHitResult _outhit)) "None" "None" 0 0 (.FaceIndex (Collision|BreakHitResult _outhit))))) (.UV (Class|GameplayStatics|FindCollisionUV _outhit))) (- (.UV (Class|GameplayStatics|FindCollisionUV (Collision|MakeHitResult false false 0.0 0.0 (+ (.Location (Collision|BreakHitResult _outhit)) (* (Math|Vector|Normalize (Math|Vector|CrossProduct (Math|Vector|Normalize (Math|Vector|CrossProduct (Math|Random|RandomUnitVectorfromStream (Math|Random|MakeRandomStream 0)) (.Normal (Collision|BreakHitResult _outhit)))) (.Normal (Collision|BreakHitResult _outhit)))) 25.0)) "0, 0, 0" "0,0,1" "0,0,1" 0 0 (.HitComponent (Collision|BreakHitResult _outhit)) "None" "None" 0 0 (.FaceIndex (Collision|BreakHitResult _outhit))))) (.UV (Class|GameplayStatics|FindCollisionUV _outhit))))) :!class /Script/Engine.MaterialInstanceDynamic)
        (Rendering|Material|SetVectorParameterValue (Variables|Default|GetBrush) "squish" (Math|Conversions|ToLinearColor(Vector) (Math|Vector|MakeVector (Math|Vector2D|DotProduct(2D) (- (.UV (Class|GameplayStatics|FindCollisionUV (Collision|MakeHitResult false false 0.0 0.0 (+ (.Location (Collision|BreakHitResult _outhit)) (* (Math|Vector|Normalize (Math|Vector|CrossProduct (Math|Random|RandomUnitVectorfromStream (Math|Random|MakeRandomStream 0)) (.Normal (Collision|BreakHitResult _outhit)))) 25.0)) "0, 0, 0" "0,0,1" "0,0,1" 0 0 (.HitComponent (Collision|BreakHitResult _outhit)) "None" "None" 0 0 (.FaceIndex (Collision|BreakHitResult _outhit))))) (.UV (Class|GameplayStatics|FindCollisionUV _outhit))) "(X=1.000000,Y=0.000000)") (Math|Vector2D|DotProduct(2D) (- (.UV (Class|GameplayStatics|FindCollisionUV (Collision|MakeHitResult false false 0.0 0.0 (+ (.Location (Collision|BreakHitResult _outhit)) (* (Math|Vector|Normalize (Math|Vector|CrossProduct (Math|Vector|Normalize (Math|Vector|CrossProduct (Math|Random|RandomUnitVectorfromStream (Math|Random|MakeRandomStream 0)) (.Normal (Collision|BreakHitResult _outhit)))) (.Normal (Collision|BreakHitResult _outhit)))) 25.0)) "0, 0, 0" "0,0,1" "0,0,1" 0 0 (.HitComponent (Collision|BreakHitResult _outhit)) "None" "None" 0 0 (.FaceIndex (Collision|BreakHitResult _outhit))))) (.UV (Class|GameplayStatics|FindCollisionUV _outhit))) "(X=0.000000,Y=1.000000)") 0.0)) :!class /Script/Engine.MaterialInstanceDynamic)
        (Rendering|DrawMaterialtoRenderTarget _returnvalue_3 (Variables|Default|GetBrush))))))

(event Input|KeyboardEvents|DebugKey1
  (params (Key :type Key%20Structure :default "None") (ActionValue :type Input%20Action%20Value%20Structure))
  (:Pressed
    (Variables|Default|SetBrush (Variables|Default|GetPositive))))

(event Input|KeyboardEvents|DebugKey2
  (params (Key :type Key%20Structure :default "None") (ActionValue :type Input%20Action%20Value%20Structure))
  (:Pressed
    (Variables|Default|SetBrush (Variables|Default|GetNegative))))

(fn ConstructionScript)